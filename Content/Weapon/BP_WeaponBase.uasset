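; Base weapon actor for BP_FirstPersonCharacter, its parent actor, handling hitscan fire, ammo and reload.
; Firing is ammo-checked and interval-gated, aims near screen center, traces from the muzzle, applies point damage and notifies via OnShoot.
; Server/MC-named events chain into montage playback, split between first-person, shadow and leg meshes for local control, third-person mesh otherwise.
; Reload refills ammo and calls OnReload on the first-person montage's notify.
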(event Custom|ServerReload
  ;[1 1 1] WeaponReload
  (CallFunction|MCReload))

(event Custom|MCReload
  ;[1 1 1] WeaponReload
  (Utilities|LocallyControlledMontagePlay (Variables|Default|GetAs%20BP%20First%20Person%20Character) "/Game/FirstPersonArms/Animations/FP_Reload_Rifle_Hip1_Montage.FP_Reload_Rifle_Hip1_Montage" "/Game/AnimStarterPack/Reload_Rifle_Hip_Montage.Reload_Rifle_Hip_Montage" "/Game/AnimStarterPack/Reload_Rifle_Hip_Montage.Reload_Rifle_Hip_Montage"
    (:通知开始时
      (Variables|Default|SetCurrentAmmo (Variables|Default|GetMaxAmmo))
      (Default|CallOnReload))))

(event Custom|FrieIntervalRelod
  (bind _returnvalue (Game|GetPlayerController 0))
  ;[1 1 1] PrimaryFrie
  (Utilities|FlowControl|DoOnce false) ; enters at Reset
)

(event Custom|SeverShooting
  (params (Direction :type Vector) (Origin :type Vector) (Content :type Player%20Controller%20Object%20Reference))
  ;[1 1 1] WeaponFire Line
  (bind _outhit (Collision|LineTraceByChannel Origin (+ Origin (* Direction (Variables|Default|GetFireRange))) "TraceTypeQuery2" false (Utilities|Array|MakeArray (Variables|Default|GetAs%20BP%20First%20Person%20Character)) "ForDuration"))
  (Variables|Default|SetOut%20Hit _outhit)
  (Utilities|FlowControl|Sequence
    (:then_0
      (CallFunction|MCFireBullet (Variables|Default|GetOut%20Hit) Direction))
    (:then_1
      (if (.bBlockingHit (Collision|BreakHitResult (Variables|Default|GetOut%20Hit)))
        (Game|Damage|ApplyPointDamage (.HitActor (Collision|BreakHitResult (Variables|Default|GetOut%20Hit))) (Variables|Default|GetBase%20Damage) (Math|Vector|GetUnitDirection(Vector) (.TraceStart (Collision|BreakHitResult (Variables|Default|GetOut%20Hit))) (.TraceEnd (Collision|BreakHitResult (Variables|Default|GetOut%20Hit)))) (Variables|Default|GetOut%20Hit) Content self)))))

(event Custom|MCFireBullet
  (params (HitResult :type Hit%20Result%20Structure) (Direction :type Vector))
  ;[1 1 1] WeaponFire
  (Utilities|LocallyControlledMontagePlay (Variables|Default|GetAs%20BP%20First%20Person%20Character) (Variables|Default|GetMontage%20to%20Play) "/Game/AnimStarterPack/Fire_Rifle_Hip_Montage.Fire_Rifle_Hip_Montage" "/Game/AnimStarterPack/Fire_Rifle_Hip_Montage.Fire_Rifle_Hip_Montage"))

(event EventBeginPlay
  ;[1 1 1] BeginPlay
  (bind _asbp_first_person_character (Utilities|Casting|CastToBP_FirstPersonCharacter (Actor|GetParentActor)))
  (bind _output_get (Variables|Default|SetAs%20BP%20First%20Person%20Character _asbp_first_person_character))
  (Actor|SetOwner _output_get)
  (Utilities|FlowControl|DelayUntilNextTick)
  (Default|CallConfigWeaponAppearence))

(event Collision|EventActorBeginOverlap
  (params (OtherActor :type Actor%20Object%20Reference))
  ;[1 1 1] BeginPlay
)

(event EventReload
  ;[1 1 1] WeaponReload
  (CallFunction|ServerReload))

(event EventPrimaryFrie
  (params (IsFring :type Boolean))
  (bind _returnvalue (Game|GetPlayerController 0))
  ;[1 1 1] PrimaryFrie
  (if IsFring
    (if (> (Variables|Default|GetCurrentAmmo) 0)
      (Utilities|FlowControl|DoOnce false
        (:Completed
          (CallFunction|SeverShooting (.WorldDirection (Class|GameplayStatics|DeprojectScreentoWorld _returnvalue (+ (/ (Viewport|GetViewportSize) 2.0) "(X=0.000000,Y=10.000000)"))) (Transformation|GetWorldLocation (Variables|Default|Getmuzzle)) _returnvalue)
          (Variables|Default|SetCurrentAmmo (- (Variables|Default|GetCurrentAmmo) 1))
          (Default|CallOnShoot)
          (Utilities|FlowControl|Delay (Variables|Default|GetFrieInterval))
          (CallFunction|FrieIntervalRelod))))))

(fn ConstructionScript)