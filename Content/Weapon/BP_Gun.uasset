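; BP_Gun is a hitscan weapon attached as a child actor of BP_FirstPersonCharacter, which it sets as owner before configuring its appearance a tick later.
; Firing deprojects a point just below screen center and passes that direction and the muzzle location to SeverShooting.
; That event line-traces on the Camera channel with debug drawing, applies point damage, and calls MCFireBullet to play first- or third-person montages depending on local control.
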(event Custom|SeverShooting
  (params (Direction :type Vector) (Origin :type Vector) (Content :type Player%20Controller%20Object%20Reference))
  ;[1 1 1] 注释
  (bind _outhit (Collision|LineTraceByChannel Origin (+ Origin (* Direction (Variables|Default|GetFireRange))) "TraceTypeQuery2" false (Utilities|Array|MakeArray (Variables|Default|GetAs%20BP%20First%20Person%20Character)) "ForDuration"))
  (Variables|Default|SetOut%20Hit _outhit)
  (Utilities|FlowControl|Sequence
    (:then_0
      (CallFunction|MCFireBullet (Variables|Default|GetOut%20Hit) Direction))
    (:then_1
      (if (.bBlockingHit (Collision|BreakHitResult (Variables|Default|GetOut%20Hit)))
        (Game|Damage|ApplyPointDamage (.HitActor (Collision|BreakHitResult (Variables|Default|GetOut%20Hit))) (Variables|Default|GetBase%20Damage) (Math|Vector|GetUnitDirection(Vector) (.TraceStart (Collision|BreakHitResult (Variables|Default|GetOut%20Hit))) (.TraceEnd (Collision|BreakHitResult (Variables|Default|GetOut%20Hit)))) (Variables|Default|GetOut%20Hit) Content self)))))

(event Custom|MCFireBullet
  (params (HitResult :type Hit%20Result%20Structure) (Direction :type Vector))
  ;[1 1 1] 注释
  (if (Pawn|IsLocallyControlled (Variables|Default|GetAs%20BP%20First%20Person%20Character))
    (Animation|Montage|MontagePlay (Components|SkeletalMesh|GetAnimInstance (Variables|/Game/FirstPerson/Blueprints/BP_FirstPersonCharacter.BP_FirstPersonCharacter_C|GetFirstPersonMesh (Variables|Default|GetAs%20BP%20First%20Person%20Character))) (Variables|Default|GetMontage%20to%20Play) 1.0 "MontageLength" 0.0 true)
    (else
      (Animation|Montage|MontagePlay (Components|SkeletalMesh|GetAnimInstance (Variables|/Game/FirstPerson/Blueprints/BP_FirstPersonCharacter.BP_FirstPersonCharacter_C|GetThirdPersonMesh (Variables|Default|GetAs%20BP%20First%20Person%20Character))) "/Game/AnimStarterPack/Fire_Rifle_Hip_Montage.Fire_Rifle_Hip_Montage" 1.0 "MontageLength" 0.0 true))))

(event EventBeginPlay
  ;[1 1 1] 注释
  (bind _asbp_first_person_character (Utilities|Casting|CastToBP_FirstPersonCharacter (Actor|GetParentActor)))
  (bind _output_get (Variables|Default|SetAs%20BP%20First%20Person%20Character _asbp_first_person_character))
  (Actor|SetOwner _output_get)
  (Utilities|FlowControl|DelayUntilNextTick)
  (Default|CallConfigWeaponAppearence))

(event Collision|EventActorBeginOverlap
  (params (OtherActor :type Actor%20Object%20Reference))
  ;[1 1 1] 注释
)

(event EventPrimaryFrie
  (params (IsFring :type Boolean))
  (bind _returnvalue (Game|GetPlayerController 0))
  ;[1 1 1] 注释
  (if IsFring
    (CallFunction|SeverShooting (.WorldDirection (Class|GameplayStatics|DeprojectScreentoWorld _returnvalue (+ (/ (Viewport|GetViewportSize) 2.0) "(X=0.000000,Y=10.000000)"))) (Transformation|GetWorldLocation (Variables|Default|Getmuzzle)) _returnvalue)))

(fn ConstructionScript)